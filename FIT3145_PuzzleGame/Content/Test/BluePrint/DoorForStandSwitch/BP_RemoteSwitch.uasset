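; BP_RemoteSwitch is a stand-on switch that unlocks a referenced door while the player character occupies its box volume.
; Box begin and end overlap events, filtered by a cast to the puzzle game character, toggle the Door's IsLocked flag when the Door reference is valid.
; The Trigger component swaps to a green material while unlocked and back to red when the character leaves and the door relocks.
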(event `self.Box.OnComponentBeginOverlap`
  (params (OverlappedComponent :type "PrimitiveComponent Object Reference") (OtherActor :type "Actor Object Reference") (OtherComp :type "PrimitiveComponent Object Reference") (OtherBodyIndex :type Integer) (bFromSweep :type Boolean) (SweepResult :type "HitResult Structure (by ref)"))
  (bind _door (`self.Door`))
  (cast `FIT3145_PuzzleGameCharacter` OtherActor)
  (`/Engine/EditorBlueprintResources/StandardMacros.IsValid` _door
    (:`Is Valid`
      (set `/Game/Test/BluePrint/DoorForStandSwitch/BP_DoorForStandSwitch.IsLocked` false _door)
      (`PrimitiveComponent.SetMaterial` (`self.Trigger`) 0 "/Game/Test/BluePrint/DoorForStandSwitch/Material_Green.Material_Green"))))

(event `self.Box.OnComponentEndOverlap`
  (params (OverlappedComponent :type "PrimitiveComponent Object Reference") (OtherActor :type "Actor Object Reference") (OtherComp :type "PrimitiveComponent Object Reference") (OtherBodyIndex :type Integer))
  (bind _door (`self.Door`))
  (cast `FIT3145_PuzzleGameCharacter` OtherActor)
  (`/Engine/EditorBlueprintResources/StandardMacros.IsValid` _door
    (:`Is Valid`
      (set `/Game/Test/BluePrint/DoorForStandSwitch/BP_DoorForStandSwitch.IsLocked` true _door)
      (`PrimitiveComponent.SetMaterial` (`self.Trigger`) 0 "/Game/Test/BluePrint/DoorForStandSwitch/Material_Red.Material_Red"))))

(fn `UserConstructionScript`)