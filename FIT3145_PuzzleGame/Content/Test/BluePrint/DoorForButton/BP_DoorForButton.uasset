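; Puzzle door that the player swings open and shut with the F key once it is unlocked, intended for use with a button.
; A box overlap by the player character enables input, shows a locked or unlocked text and, if unlocked, opens a Gate.
; F passes through the Gate to a FlipFlop that plays or reverses a Timeline driving door yaw.
; IsLocked is only read here, never set.
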(event `Key|F`
  (params (Key :type "Key Structure"))
  (:`Pressed`
    (if (`self.IsLocked`)
      (`KismetSystemLibrary.PrintString` "You need to press button to unlock the door")
      (else
        (`KismetSystemLibrary.PrintString` "The door is unlocked")
        (`/Engine/EditorBlueprintResources/StandardMacros.Gate` true :!label _label
          (:`Exit`
            (`/Engine/EditorBlueprintResources/StandardMacros.FlipFlop`
              (:`A`
                (bind (_direction _newtrack_0) (`Timeline|Timeline_0` :!label _label_2)
                  (:`Update`
                    (`SceneComponent.K2_SetRelativeRotation` (`self.Door`) (`KismetMathLibrary.MakeRotator` 0.0 0.0 _newtrack_0) false false))))
              (:`B`
                (goto _label_2 :!via `Reverse`)))))))))

(event `Key|E`
  (params (Key :type "Key Structure")))

(event `self.Box.OnComponentBeginOverlap`
  (params (OverlappedComponent :type "PrimitiveComponent Object Reference") (OtherActor :type "Actor Object Reference") (OtherComp :type "PrimitiveComponent Object Reference") (OtherBodyIndex :type Integer) (bFromSweep :type Boolean) (SweepResult :type "HitResult Structure (by ref)"))
  (cast `FIT3145_PuzzleGameCharacter` OtherActor)
  (`self.EnableInput` (`GameplayStatics.GetPlayerController` 0))
  (if (`self.IsLocked`)
    (`SceneComponent.SetVisibility` (`self.TextRender1`) true false)
    (else
      (`SceneComponent.SetVisibility` (`self.TextRender`) true false)
      (goto _label :!via `Open`))))

(event `self.Box.OnComponentEndOverlap`
  (params (OverlappedComponent :type "PrimitiveComponent Object Reference") (OtherActor :type "Actor Object Reference") (OtherComp :type "PrimitiveComponent Object Reference") (OtherBodyIndex :type Integer))
  (cast `FIT3145_PuzzleGameCharacter` OtherActor)
  (`self.DisableInput` (`GameplayStatics.GetPlayerController` 0))
  (`SceneComponent.SetVisibility` (`self.TextRender1`) false false)
  (`SceneComponent.SetVisibility` (`self.TextRender`) false false)
  (goto _label :!via `Close`))

(fn `UserConstructionScript`)