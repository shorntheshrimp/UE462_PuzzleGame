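; BP_Button is an interactable button that unlocks a BP_DoorForButton when the player presses F nearby.
; Box overlap with the player character enables input, shows a text prompt and opens a gate; leaving closes the gate.
; F passes through the gate and clears IsLocked on the first door found by GetAllActorsOfClass.
; The text-hiding node is unconnected, so the prompt stays visible, and end overlap leaves input enabled.
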(event `Key|F`
  (params (Key :type "Key Structure"))
  (:`Pressed`
    (`KismetSystemLibrary.PrintString` "You have pressed the button")
    (`/Engine/EditorBlueprintResources/StandardMacros.Gate` true :!label _label
      (:`Exit`
        (bind _outactors (`GameplayStatics.GetAllActorsOfClass` "/Game/Test/BluePrint/DoorForButton/BP_DoorForButton.BP_DoorForButton_C"))
        (set `/Game/Test/BluePrint/DoorForButton/BP_DoorForButton.IsLocked` false (`|GetArrayItem` _outactors))))))

(event `Key|E`
  (params (Key :type "Key Structure")))

(event `self.Box.OnComponentBeginOverlap`
  (params (OverlappedComponent :type "PrimitiveComponent Object Reference") (OtherActor :type "Actor Object Reference") (OtherComp :type "PrimitiveComponent Object Reference") (OtherBodyIndex :type Integer) (bFromSweep :type Boolean) (SweepResult :type "HitResult Structure (by ref)"))
  (cast `FIT3145_PuzzleGameCharacter` OtherActor)
  (`KismetSystemLibrary.PrintString` "Press \"F\" press button")
  (`self.EnableInput` (`GameplayStatics.GetPlayerController` 0))
  (`SceneComponent.SetVisibility` (`self.TextRender`) true false)
  (goto _label :!via `Open`))

(event `self.Box.OnComponentEndOverlap`
  (params (OverlappedComponent :type "PrimitiveComponent Object Reference") (OtherActor :type "Actor Object Reference") (OtherComp :type "PrimitiveComponent Object Reference") (OtherBodyIndex :type Integer))
  (cast `FIT3145_PuzzleGameCharacter` OtherActor)
  (`self.EnableInput` (`GameplayStatics.GetPlayerController` 0))
  (goto _label :!via `Close`))

(fn `UserConstructionScript`)