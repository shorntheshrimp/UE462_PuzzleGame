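; BP_Light1 is a puzzle light that the player switches on to help unlock a linked Door.
; Its Box overlap enables input, shows a text prompt and opens a gate for the F key while the character is near an unlit light.
; Pressing F turns on the SpotLight, then checks every BP_Light1 in the level, unlocking the Door only when all are lit.
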(event `Key|F`
  (params (Key :type "Key Structure"))
  (bind _door (`self.Door`))
  (bind _door_2 (`self.Door`))
  (:`Pressed`
    (`/Engine/EditorBlueprintResources/StandardMacros.Gate` true :!label _label
      (:`Exit`
        (`SceneComponent.SetVisibility` (`self.SpotLight`) true false)
        (`SceneComponent.SetVisibility` (`self.TextRender`) false false)
        (set `self.IfOpenLight` true)
        (bind _outactors (`GameplayStatics.GetAllActorsOfClass` "BP_Light1_C"))
        (for _array_element _outactors
          (if (`/Game/Test/BluePrint/DoorLight/BP_Light1.IfOpenLight` _array_element)
            (set `self.IfOpenDoor` true)
            (else
              (set `self.IfOpenDoor` false)
              (break))))
        (if (`self.IfOpenDoor`)
          (`/Engine/EditorBlueprintResources/StandardMacros.IsValid` _door
            (:`Is Valid`
              (set `/Game/Test/BluePrint/DoorLight/BP_DoorLight.IsLocked` false _door)))
          (else
            (`/Engine/EditorBlueprintResources/StandardMacros.IsValid` _door_2
              (:`Is Valid`
                (set `/Game/Test/BluePrint/DoorLight/BP_DoorLight.IsLocked` true _door_2)))))))))

(event `self.Box.OnComponentBeginOverlap`
  (params (OverlappedComponent :type "PrimitiveComponent Object Reference") (OtherActor :type "Actor Object Reference") (OtherComp :type "PrimitiveComponent Object Reference") (OtherBodyIndex :type Integer) (bFromSweep :type Boolean) (SweepResult :type "HitResult Structure (by ref)"))
  (cast `FIT3145_PuzzleGameCharacter` OtherActor)
  (if (not (`self.IfOpenLight`))
    (`self.EnableInput` (`GameplayStatics.GetPlayerController` 0))
    (`SceneComponent.SetVisibility` (`self.TextRender`) true false)
    (goto _label :!via `Open`)))

(event `self.Box.OnComponentEndOverlap`
  (params (OverlappedComponent :type "PrimitiveComponent Object Reference") (OtherActor :type "Actor Object Reference") (OtherComp :type "PrimitiveComponent Object Reference") (OtherBodyIndex :type Integer))
  (cast `FIT3145_PuzzleGameCharacter` OtherActor)
  (`self.DisableInput` (`GameplayStatics.GetPlayerController` 0))
  (`SceneComponent.SetVisibility` (`self.TextRender`) false false)
  (goto _label :!via `Close`))

(fn `UserConstructionScript`)