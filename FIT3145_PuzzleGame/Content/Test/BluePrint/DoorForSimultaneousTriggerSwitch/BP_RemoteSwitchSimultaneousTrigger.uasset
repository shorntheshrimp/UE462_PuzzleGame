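; Pressure switch for a puzzle door that unlocks when every switch of this class in the level is triggered.
; The player character's first overlap latches the switch, then it checks all instances and sets its linked Door's lock.
; Any end overlap relocks that Door, while the trigger flag stays set because its reset logic is disconnected.
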(event `self.Box.OnComponentBeginOverlap`
  (params (OverlappedComponent :type "PrimitiveComponent Object Reference") (OtherActor :type "Actor Object Reference") (OtherComp :type "PrimitiveComponent Object Reference") (OtherBodyIndex :type Integer) (bFromSweep :type Boolean) (SweepResult :type "HitResult Structure (by ref)"))
  (bind _door (`self.Door`))
  (bind _door_2 (`self.Door`))
  (cast `FIT3145_PuzzleGameCharacter` OtherActor)
  (if (not (`self.IsTriggerSwitch`))
    (set `self.IsTriggerSwitch` true)
    (bind _outactors (`GameplayStatics.GetAllActorsOfClass` "BP_RemoteSwitchSimultaneousTrigger_C"))
    (for _array_element _outactors
      (if (`/Game/Test/BluePrint/DoorForSimultaneousTriggerSwitch/BP_RemoteSwitchSimultaneousTrigger.IsTriggerSwitch` _array_element)
        (set `self.IsOpenDoor` true)
        (set `self.IsStanding` true)
        (else
          (set `self.IsOpenDoor` false)
          (set `self.IsStanding` false)
          (break))))
    (if (`self.IsOpenDoor`) :!label _label
      (`/Engine/EditorBlueprintResources/StandardMacros.IsValid` _door
        (:`Is Valid`
          (set `/Game/Test/BluePrint/DoorForSimultaneousTriggerSwitch/BP_DoorForSimultaneousTriggerSwitch.IsLocked` false _door)))
      (else
        (`/Engine/EditorBlueprintResources/StandardMacros.IsValid` _door_2
          (:`Is Valid`
            (set `/Game/Test/BluePrint/DoorForSimultaneousTriggerSwitch/BP_DoorForSimultaneousTriggerSwitch.IsLocked` true _door_2)))))))

(event `self.Box.OnComponentEndOverlap`
  (params (OverlappedComponent :type "PrimitiveComponent Object Reference") (OtherActor :type "Actor Object Reference") (OtherComp :type "PrimitiveComponent Object Reference") (OtherBodyIndex :type Integer))
  (set `self.IsOpenDoor` false)
  (goto _label))

(fn `UserConstructionScript`)